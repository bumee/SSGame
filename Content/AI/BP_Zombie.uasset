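; BP_Zombie is a zombie AI Blueprint that loads the BB_AIJumping blackboard on BeginPlay.
; ChasePlace writes a random reachable point near the first BP_AITarget into MoveLocation and runs BT_AIJumping, though nothing here calls it.
; CheckFindPlayer tests whether its own location projects inside the first player's viewport, with no line-of-sight check.
; Tick calls that test every frame but discards the result.
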(event EventBeginPlay
  (bind _blackboardcomponent (Class|AIController|UseBlackboard "/Game/AI/BB_AIJumping.BB_AIJumping"))
  (Variables|Default|SetCurrentBlackBoard _blackboardcomponent))

(event EventTick
  (params (DeltaSeconds :type Float%20%28single-precision%29))
  (CallFunction|CheckFindPlayer))

(fn ConstructionScript)

(fn ChasePlace
  (bind _outactors (Actor|GetAllActorsOfClass "/Game/AI/BP_AITarget.BP_AITarget_C"))
  (AI|Components|Blackboard|SetValueasVector (Variables|Default|GetCurrentBlackBoard) (Utilities|Name|MakeLiteralName "MoveLocation") (.RandomLocation (AI|Navigation|GetRandomReachablePointinRadius (Transformation|GetActorLocation (Utilities|Array|Get(acopy) _outactors)) 25.0 0 0)))
  (AI|RunBehaviorTree "/Game/AI/BT_AIJumping.BT_AIJumping"))

(fn CheckFindPlayer
  (bind _returnvalue (Game|GetPlayerController 0))
  (bind _returnvalue_2 (Transformation|GetActorLocation))
  (bind _returnvalue_3 (Viewport|GetViewportSize))
  (bind _screenlocation (Class|PlayerController|ProjectWorldLocationtoScreen _returnvalue _returnvalue_2 false))
  (return (Math|Boolean|ANDBoolean (> (.x _screenlocation) 0.0) (> (.y _screenlocation) 0.0) (< (.x _screenlocation) (.x _returnvalue_3)) (< (.y _screenlocation) (.y _returnvalue_3)))))